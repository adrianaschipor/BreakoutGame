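; B_GameState is a game state Blueprint that tracks the player's score and lives.
; IncreaseScore adds one to Score, and DecreaseLives subtracts one from Lives and returns the new count.
; Every Tick prints ScoreString followed by the current Score as on-screen debug text, while Lives is never displayed.
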(event EventBeginPlay)

(event EventTick
  (params (DeltaSeconds :type Float%20%28single-precision%29))
  (Development|PrintText (Utilities|Text|ToText(String) (Utilities|String|Append (Variables|Default|GetScoreString) (Utilities|String|ToString(Text) (Utilities|Text|ToText(Integer) (Variables|Default|GetScore)))))))

(fn ConstructionScript)

(fn IncreaseScore
  (Variables|Default|SetScore (+ (Variables|Default|GetScore) 1)))

(fn DecreaseLives
  (bind _output_get (Variables|Default|SetLives (- (Variables|Default|GetLives) 1)))
  (return _output_get))