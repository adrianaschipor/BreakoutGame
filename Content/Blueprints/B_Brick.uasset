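; B_Brick is a brick actor that reacts to being hit by a ball.
; A component hit from a B_Ball decrements its Lifespan by one.
; Logic to destroy the brick at zero Lifespan and increase the B_GameState score exists but is disconnected, so it never runs.
; A separate DecreaseLifespan function duplicates the decrement, and the hit event does not call it.
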(event OnComponentHit(C_Brick)
  (params (HitComponent :type Primitive%20Component%20Object%20Reference) (OtherActor :type Actor%20Object%20Reference) (OtherComp :type Primitive%20Component%20Object%20Reference) (NormalImpulse :type Vector :default "0, 0, 0") (Hit :type Hit%20Result%20Structure%20%28by%20ref%29))
  ;[1 1 1] Handle Brick collision
  (Utilities|Casting|CastToB_Ball OtherActor)
  (bind _output_get (Variables|Default|Setlifespan (- (Variables|Default|Getlifespan) 1))))

(fn ConstructionScript)

(fn DecreaseLifespan
  (Variables|Default|Setlifespan (- (Variables|Default|Getlifespan) 1)))